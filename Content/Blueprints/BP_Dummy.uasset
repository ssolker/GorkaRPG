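; BP_Dummy is a target dummy character that can be stealth-assassinated.
; An overlap radius shows a prompt widget to BP_ThirdPersonCharacter, and Tick keeps it turned toward the player camera.
; StealthBackAssassin plays the death montage, schedules a delayed mesh ragdoll, hides the prompt and returns the AssassinRef location and dummy rotation, presumably for placing the attacker.
; It also draws a debug sphere at that reference point.
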(event `self.ReceiveTick`
  (params (DeltaSeconds :type "Float (single-precision)"))
  (`SceneComponent.K2_SetWorldRotation` (`self.AssassinateWidget`) (`KismetMathLibrary.FindLookAtRotation` (`SceneComponent.K2_GetComponentLocation` (`self.AssassinateWidget`)) (`SceneComponent.K2_GetComponentLocation` (`PlayerCameraManager.TransformComponent` (`GameplayStatics.GetPlayerCameraManager` 0)))) false false))

(event `Ragdoll`
  ;[1 1 1] Ragdoll after death animation
  (`KismetSystemLibrary.Delay` 4.5)
  (`PrimitiveComponent.SetSimulatePhysics` (`self.Mesh`) true))

(event `self.AssassinationRadius.OnComponentBeginOverlap`
  (params (OverlappedComponent :type "PrimitiveComponent Object Reference") (OtherActor :type "Actor Object Reference") (OtherComp :type "PrimitiveComponent Object Reference") (OtherBodyIndex :type Integer) (bFromSweep :type Boolean) (SweepResult :type "HitResult Structure (by ref)"))
  (cast `/Game/ThirdPerson/Blueprints/BP_ThirdPersonCharacter` OtherActor)
  (`SceneComponent.SetVisibility` (`self.AssassinateWidget`) true false))

(event `self.AssassinationRadius.OnComponentEndOverlap`
  (params (OverlappedComponent :type "PrimitiveComponent Object Reference") (OtherActor :type "Actor Object Reference") (OtherComp :type "PrimitiveComponent Object Reference") (OtherBodyIndex :type Integer))
  (cast `/Game/ThirdPerson/Blueprints/BP_ThirdPersonCharacter` OtherActor)
  (`SceneComponent.SetVisibility` (`self.AssassinateWidget`) false false))

(fn `StealthBackAssassin`
  (returns (`Ref Location` :type "Vector Structure") (`Assassin Rotation` :type "Rotator Structure"))
  (bind _returnvalue (`SceneComponent.K2_GetComponentLocation` (`self.AssassinRef`)))
  (`self.PlayAnimMontage` "/Game/Characters/RPG_Character/Animations/Assassination/AM_StealthAssassinationDeath_UE_Montage.AM_StealthAssassinationDeath_UE_Montage")
  (`self.Ragdoll`)
  (`SceneComponent.SetVisibility` (`self.AssassinateWidget`) false false)
  (`KismetSystemLibrary.DrawDebugSphere` _returnvalue 20.0 12 (struct :`R` 1.0 :`B` 0.023868 :`A` 1.0) 2.0)
  (return _returnvalue (`self.K2_GetActorRotation`)))

(fn `UserConstructionScript`)