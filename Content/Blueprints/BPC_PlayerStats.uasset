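; Player stats component for BP_ThirdPersonCharacter that tracks health, stamina, XP and level.
; It caches its owning character on BeginPlay, and most stat functions push values straight into that character's HUD widget.
; Health and stamina increases cap at their maximums, while the decrease functions report depletion.
; Reaching MaxXP raises the level, derives a new threshold from current XP and resets XP.
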(event `self.ReceiveBeginPlay`
  (bind _asbp_third_person_character (cast `/Game/ThirdPerson/Blueprints/BP_ThirdPersonCharacter` (`self.GetOwner`)))
  (set `self.PlayerCharacterBP` _asbp_third_person_character))

(fn `DecreaseHealth`
  (params (Damage :type "Float (double-precision)"))
  (returns (isPlayerDead :type Boolean))
  (bind _returnvalue (- (`self.CurrentHealth`) Damage))
  (bind _hudwidget (`/Game/ThirdPerson/Blueprints/BP_ThirdPersonCharacter.HUDWidget` (`self.PlayerCharacterBP`)))
  (if (< _returnvalue 0.0)
    (set `self.CurrentHealth` 0.0)
    (else
      (bind _output_get (set `self.CurrentHealth` _returnvalue))))
  (`ProgressBar.SetPercent` (`/Game/UI/WB_HUD.HealthBar` _hudwidget) (/ _output_get (`self.MaxHealth`)))
  (`TextBlock.SetText` (`/Game/UI/WB_HUD.HealthText` _hudwidget) (`KismetTextLibrary.Conv_DoubleToText` (`self.CurrentHealth`) "HalfToEven"))
  (return (<= (`self.CurrentHealth`) 0.0)))

(fn `DecreaseStamina`
  (params (StaminaUsed :type "Float (double-precision)"))
  (returns (isStaminaDepleted :type Boolean))
  (set `self.CurrentStamina` (- (`self.CurrentStamina`) StaminaUsed))
  (`ProgressBar.SetPercent` (`/Game/UI/WB_HUD.StaminaBar` (`/Game/ThirdPerson/Blueprints/BP_ThirdPersonCharacter.HUDWidget` (`self.PlayerCharacterBP`))) (/ (`self.CurrentStamina`) (`self.MaxStamina`)))
  (return (<= (`self.CurrentStamina`) 0.0)))

(fn `IncreaseHealth`
  (params (HealthIncrement :type "Float (double-precision)"))
  (bind _maxhealth (`self.MaxHealth`))
  (bind _hudwidget (`/Game/ThirdPerson/Blueprints/BP_ThirdPersonCharacter.HUDWidget` (`self.PlayerCharacterBP`)))
  (set `self.CurrentHealth` (+ (`self.CurrentHealth`) HealthIncrement))
  (if (> (`self.CurrentHealth`) _maxhealth)
    (set `self.CurrentHealth` _maxhealth))
  (`ProgressBar.SetPercent` (`/Game/UI/WB_HUD.HealthBar` _hudwidget) (/ (`self.CurrentHealth`) (`self.MaxHealth`)))
  (`TextBlock.SetText` (`/Game/UI/WB_HUD.HealthText` _hudwidget) (`KismetTextLibrary.Conv_DoubleToText` (`self.CurrentHealth`) "HalfToEven")))

(fn `IncreaseLevel`
  (params (LevelIncrease :type Integer))
  (set `self.Level` (+ (`self.Level`) LevelIncrease))
  (set `self.MaxXP` (+ (`self.XP`) 150.0))
  (set `self.XP` 0.0)
  (`TextBlock.SetText` (`/Game/UI/WB_HUD.LevelText` (`/Game/ThirdPerson/Blueprints/BP_ThirdPersonCharacter.HUDWidget` (`self.PlayerCharacterBP`))) (`KismetTextLibrary.Conv_IntToText` (`self.Level`))))

(fn `IncreaseMaxHealth`
  (params (HealthIncrement :type "Float (double-precision)"))
  (bind _hudwidget (`/Game/ThirdPerson/Blueprints/BP_ThirdPersonCharacter.HUDWidget` (`self.PlayerCharacterBP`)))
  (set `self.MaxHealth` (+ (`self.MaxHealth`) HealthIncrement))
  (`ProgressBar.SetPercent` (`/Game/UI/WB_HUD.HealthBar` _hudwidget) (/ (`self.CurrentHealth`) (`self.MaxHealth`)))
  (`TextBlock.SetText` (`/Game/UI/WB_HUD.HealthText` _hudwidget) (`KismetTextLibrary.Conv_DoubleToText` (`self.CurrentHealth`) "HalfToEven")))

(fn `IncreaseMaxStamina`
  (params (StaminaIncrement :type "Float (double-precision)"))
  (set `self.MaxStamina` (+ (`self.MaxStamina`) StaminaIncrement)))

(fn `IncreaseStamina`
  (params (StaminaIncrement :type "Float (double-precision)"))
  (bind _maxstamina (`self.MaxStamina`))
  (set `self.CurrentStamina` (+ (`self.CurrentStamina`) StaminaIncrement))
  (if (> (`self.CurrentStamina`) _maxstamina)
    (set `self.CurrentStamina` _maxstamina))
  (`ProgressBar.SetPercent` (`/Game/UI/WB_HUD.StaminaBar` (`/Game/ThirdPerson/Blueprints/BP_ThirdPersonCharacter.HUDWidget` (`self.PlayerCharacterBP`))) (/ (`self.CurrentStamina`) (`self.MaxStamina`))))

(fn `IncreaseXP`
  (params (XP :type "Float (double-precision)"))
  (set `self.XP` (+ XP (`self.XP`)))
  (`ProgressBar.SetPercent` (`/Game/UI/WB_HUD.XPBar` (`/Game/ThirdPerson/Blueprints/BP_ThirdPersonCharacter.HUDWidget` (`self.PlayerCharacterBP`))) (/ (`self.XP`) (`self.MaxXP`)))
  (if (>= (`self.XP`) (`self.MaxXP`))
    (`self.IncreaseLevel` 1)
    (`ProgressBar.SetPercent` (`/Game/UI/WB_HUD.XPBar` (`/Game/ThirdPerson/Blueprints/BP_ThirdPersonCharacter.HUDWidget` (`self.PlayerCharacterBP`))) (/ (`self.XP`) (`self.MaxXP`)))))